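; Boost pad actor that launches overlapping sedan vehicles forward at a configurable speed.
; On overlap, a sequence casts the other actor to each sedan class and overwrites its mesh physics velocity along its forward vector, scaled from SetSpeedMpH.
; A TheSedan overlap also plays Duration, which drives nothing in this graph.
; BeginPlay caches a TheSedan reference that the overlap logic does not use.
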(event EventBeginPlay
  (bind _returnvalue (Actor|GetActorOfClass "/Game/tim/player/TheSedan.TheSedan_C"))
  (Variables|Default|SetSedan _returnvalue))

(event Collision|EventActorBeginOverlap
  (params (OtherActor :type Actor%20Object%20Reference))
  (Utilities|FlowControl|Sequence
    (:then_0
      (Utilities|Casting|CastToTheSedan OtherActor)
      (Timeline|Duration Play))
    (:then_1
      (bind _assedan_child_1 (Utilities|Casting|CastToSedan_Child_1 OtherActor))
      (Physics|SetPhysicsLinearVelocity (Variables|/Script/PhysXVehicles.WheeledVehicle|GetMesh _assedan_child_1) (* (* (Transformation|GetActorForwardVector _assedan_child_1) 28) (Variables|Default|GetSet%20Speed%20MpH)) false "None"))
    (:then_2
      (bind _assedan_child_2 (Utilities|Casting|CastToSedan_Child_2 OtherActor))
      (Physics|SetPhysicsLinearVelocity (Variables|/Script/PhysXVehicles.WheeledVehicle|GetMesh _assedan_child_2) (* (* (Transformation|GetActorForwardVector _assedan_child_2) 28) (Variables|Default|GetSet%20Speed%20MpH)) false "None"))
    (:then_3
      (bind _assedan_child_3 (Utilities|Casting|CastToSedan_Child_3 OtherActor))
      (Physics|SetPhysicsLinearVelocity (Variables|/Script/PhysXVehicles.WheeledVehicle|GetMesh _assedan_child_3) (* (* (Transformation|GetActorForwardVector _assedan_child_3) 28) (Variables|Default|GetSet%20Speed%20MpH)) false "None"))
    (:then_4
      (bind _assedan_child_4 (Utilities|Casting|CastToSedan_Child_4 OtherActor))
      (Physics|SetPhysicsLinearVelocity (Variables|/Script/PhysXVehicles.WheeledVehicle|GetMesh _assedan_child_4) (* (* (Transformation|GetActorForwardVector _assedan_child_4) 28) (Variables|Default|GetSet%20Speed%20MpH)) false "None"))
    (:then_5
      (bind _asthe_sedan (Utilities|Casting|CastToTheSedan OtherActor))
      (Physics|SetPhysicsLinearVelocity (Variables|/Script/PhysXVehicles.WheeledVehicle|GetMesh _asthe_sedan) (* (* (Transformation|GetActorForwardVector _asthe_sedan) 28) (Variables|Default|GetSet%20Speed%20MpH)) false "None"))
    (:then_6
      (bind _assedan (Utilities|Casting|CastToSedan OtherActor))
      (Physics|SetPhysicsLinearVelocity (Variables|/Script/PhysXVehicles.WheeledVehicle|GetMesh _assedan) (* (* (Transformation|GetActorForwardVector _assedan) 28) (Variables|Default|GetSet%20Speed%20MpH)) false "None"))))

(fn ConstructionScript)